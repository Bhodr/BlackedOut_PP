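; BP_Portal_Enter is an entrance portal that teleports the third-person player character to its paired exit portal.
; On BeginPlay it searches all BP_Portal_Out actors and stores the one with a matching PortalNumber as ExitPortal.
; When its Sphere component is hit by BP_ThirdPersonCharacter, it teleports the character slightly above that exit with zeroed rotation.
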(event `self.Sphere.OnComponentHit`
  (params (HitComponent :type "PrimitiveComponent Object Reference") (OtherActor :type "Actor Object Reference") (OtherComp :type "PrimitiveComponent Object Reference") (NormalImpulse :type "Vector Structure") (Hit :type "HitResult Structure (by ref)"))
  (bind _asbp_third_person_character (cast `/Game/ThirdPerson/Blueprints/BP_ThirdPersonCharacter` OtherActor))
  (bind _output_get (set `self.TPCharacter` _asbp_third_person_character))
  (`self.K2_TeleportTo` :`self` _output_get :`DestLocation` (+ (`self.K2_GetActorLocation` (`self.ExitPortal`)) (0.0 0.0 100.0))))

(event `self.ReceiveBeginPlay`
  (bind _outactors (`GameplayStatics.GetAllActorsOfClass` "/Game/BP/BP_Portal_Out.BP_Portal_Out_C"))
  (for _array_element _outactors
    (`/Engine/EditorBlueprintResources/StandardMacros.IsValid` _array_element
      (:`Is Valid`
        (if (== (`/Game/BP/BP_Portal_Out.PortalNumber` _array_element) (`self.PortalNumber`))
          (set `self.ExitPortal` _array_element))))))

(fn `UserConstructionScript`)